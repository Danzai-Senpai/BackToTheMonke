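; FPSCharacter is a first-person Character Blueprint that handles player movement, camera look and jumping through input axis and action events.
; Forward and right movement use a yaw-only rotator from the control rotation, so camera pitch does not affect direction.
; Mouse axes feed controller yaw and pitch directly, while gamepad look scales by a Sensibility variable and world delta seconds for frame-rate independence.
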(event `InputAxis|MouseX`
  (params (AxisValue :type "Float (single-precision)"))
  ;[0 0.5 1] Nodes Of Movement
  ;;[0 1 0.02733] Camera (Mouse)
  (`self.AddControllerYawInput` AxisValue) ; Yaw é o representação da Rotação no eixo X
)

(event `InputAxis|MouseY`
  (params (AxisValue :type "Float (single-precision)"))
  ;[0 0.5 1] Nodes Of Movement
  ;;[0 1 0.02733] Camera (Mouse)
  (`self.AddControllerPitchInput` AxisValue))

(event `InputAxis|MoveForward`
  (params (AxisValue :type "Float (single-precision)"))
  ;[0 0.5 1] Nodes Of Movement
  ;;[0 1 0.02745] Movement Player
  (`self.AddMovementInput` (`KismetMathLibrary.GetForwardVector` (`KismetMathLibrary.MakeRotator` 0.0 0.0 (.yaw (`self.GetControlRotation`)))) AxisValue) ; Adicionar informações de Movimento
)

(event `InputAction|Jump`
  (params (Key :type "Key Structure"))
  ;[0 0.5 1] Nodes Of Movement
  ;;[0 1 0.02745] Jump Player
  (:`Pressed`
    (`self.Jump`))
  (:`Released`
    (`self.StopJumping`)))

(event `InputAxis|GamepadX`
  (params (AxisValue :type "Float (single-precision)"))
  ;[0 0.5 1] Nodes Of Movement
  ;;[0 1 0.02745] Camera (Gamepad)
  (`self.AddControllerYawInput` (* AxisValue (`self.Sensibility`) (`GameplayStatics.GetWorldDeltaSeconds`))))

(event `InputAxis|MoveRight`
  (params (AxisValue :type "Float (single-precision)"))
  ;[0 0.5 1] Nodes Of Movement
  ;;[0 1 0.02745] Movement Player
  (`self.AddMovementInput` (`KismetMathLibrary.GetRightVector` (`KismetMathLibrary.MakeRotator` 0.0 0.0 (.yaw (`self.GetControlRotation`)))) AxisValue))

(event `InputAxis|GamepadY`
  (params (AxisValue :type "Float (single-precision)"))
  ;[0 0.5 1] Nodes Of Movement
  ;;[0 1 0.02745] Camera (Gamepad)
  (`self.AddControllerPitchInput` (* AxisValue (`self.Sensibility`) (`GameplayStatics.GetWorldDeltaSeconds`))))

(fn `UserConstructionScript`)